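; BP_Chest is an interactable storage chest with its own inventory that opens and closes as the player moves near it.
; Entering the EntryBox shows the chest inventory and turns the player's item text off; leaving the ExitBox hides it, calls LeaveChest and restores the text.
; Wrapper functions forward adding items, moving the slot selector, checking free space and removing the selected item for transfer to the BPCMPInventorySystem component.
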(event `self.Exit Box.OnComponentEndOverlap`
  (params (OverlappedComponent :type "PrimitiveComponent Object Reference") (OtherActor :type "Actor Object Reference") (OtherComp :type "PrimitiveComponent Object Reference") (OtherBodyIndex :type Integer))
  (if (`self.ActorHasTag` OtherActor "Player")
    (`self.CloseChest`)
    (bind _asbp_player_character (cast `/Game/GEP/Blueprints/Essentials/BP_PlayerCharacter` OtherActor))
    (`/Game/GEP/Blueprints/Essentials/BP_PlayerCharacter.LeaveChest` _asbp_player_character)
    (`/Game/GEP/Blueprints/Essentials/BP_PlayerCharacter.ItemTextOn` _asbp_player_character)))

(event `self.Entry Box.OnComponentBeginOverlap`
  (params (OverlappedComponent :type "PrimitiveComponent Object Reference") (OtherActor :type "Actor Object Reference") (OtherComp :type "PrimitiveComponent Object Reference") (OtherBodyIndex :type Integer) (bFromSweep :type Boolean) (SweepResult :type "HitResult Structure (by ref)"))
  (if (`self.ActorHasTag` OtherActor "Player")
    (`self.OpenChest`)
    (bind _asbp_player_character (cast `/Game/GEP/Blueprints/Essentials/BP_PlayerCharacter` OtherActor))
    (`/Game/GEP/Blueprints/Essentials/BP_PlayerCharacter.ItemTextOff` _asbp_player_character)))

(fn `AddItem`
  (params (ItemId :type Integer))
  (`/Game/GEP/Blueprints/Systems/BP_CMP_InventorySystem.AddItem` (`self.BP_CMP_InventorySystem`) ItemId))

(fn `CheckIfFreeSpace`
  (params (item_id :type Integer))
  (returns (free_space_out :type Boolean))
  (bind _free_space_out (`/Game/GEP/Blueprints/Systems/BP_CMP_InventorySystem.Check if Free Space` (`self.BP_CMP_InventorySystem`) item_id))
  (return _free_space_out))

(fn `CloseChest`
  (`/Game/GEP/Blueprints/Systems/BP_CMP_InventorySystem.InventoryOff` (`self.BP_CMP_InventorySystem`)))

(fn `MoveChestSlotSelector`
  (params (Direction :type Integer))
  (`/Game/GEP/Blueprints/Systems/BP_CMP_InventorySystem.MoveSlotSelector` (`self.BP_CMP_InventorySystem`) Direction))

(fn `OpenChest`
  (`/Game/GEP/Blueprints/Systems/BP_CMP_InventorySystem.InventoryOn` (`self.BP_CMP_InventorySystem`)))

(fn `TransferItem`
  (returns (item_id :type Integer))
  (bind _bp_cmp_inventorysystem (`self.BP_CMP_InventorySystem`))
  (bind _item_id (`/Game/GEP/Blueprints/Systems/BP_CMP_InventorySystem.GetCurrentItemId` _bp_cmp_inventorysystem))
  (`/Game/GEP/Blueprints/Systems/BP_CMP_InventorySystem.RemoveItem` _bp_cmp_inventorysystem)
  (return _item_id))

(fn `UserConstructionScript`)