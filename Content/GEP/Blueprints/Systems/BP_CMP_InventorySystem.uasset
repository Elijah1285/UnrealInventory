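; Inventory component for a block-building game, serving as either a player inventory or a chest through a Chest flag that picks the widget panel.
; An array of slot structs holds item IDs and counts, stacking items up to per-type limits.
; Adding or removing items refreshes icons, count labels and the next free slot.
; A grid selector chooses the current slot, whose ID determines which actor PlaceItem spawns.
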(event `self.ReceiveBeginPlay`
  (bind _inv_panel (`self.inv_panel`))
  (bind _chest_panel (`self.chest_panel`))
  (if (`self.chest`)
    (bind _returnvalue (`|CreateWidget` "/Game/GEP/Blueprints/UI/WGT_BP_ChestPanel.WGT_BP_ChestPanel_C"))
    (set `self.chest_panel` _returnvalue)
    (set `self.inv_slots` (`|MakeArray` (`/Game/GEP/Blueprints/UI/WGT_BP_ChestPanel.slot_1` _chest_panel) (`/Game/GEP/Blueprints/UI/WGT_BP_ChestPanel.slot_2` _chest_panel) (`/Game/GEP/Blueprints/UI/WGT_BP_ChestPanel.slot_3` _chest_panel) (`/Game/GEP/Blueprints/UI/WGT_BP_ChestPanel.slot_4` _chest_panel) (`/Game/GEP/Blueprints/UI/WGT_BP_ChestPanel.slot_5` _chest_panel) (`/Game/GEP/Blueprints/UI/WGT_BP_ChestPanel.slot_6` _chest_panel) (`/Game/GEP/Blueprints/UI/WGT_BP_ChestPanel.slot_7` _chest_panel) (`/Game/GEP/Blueprints/UI/WGT_BP_ChestPanel.slot_8` _chest_panel) (`/Game/GEP/Blueprints/UI/WGT_BP_ChestPanel.slot_9` _chest_panel)))
    (set `self.slot_counts` (`|MakeArray` (`/Game/GEP/Blueprints/UI/WGT_BP_ChestPanel.slot_1_count` _chest_panel) (`/Game/GEP/Blueprints/UI/WGT_BP_ChestPanel.slot_2_count` _chest_panel) (`/Game/GEP/Blueprints/UI/WGT_BP_ChestPanel.slot_3_count` _chest_panel) (`/Game/GEP/Blueprints/UI/WGT_BP_ChestPanel.slot_4_count` _chest_panel) (`/Game/GEP/Blueprints/UI/WGT_BP_ChestPanel.slot_5_count` _chest_panel) (`/Game/GEP/Blueprints/UI/WGT_BP_ChestPanel.slot_6_count` _chest_panel) (`/Game/GEP/Blueprints/UI/WGT_BP_ChestPanel.slot_7_count` _chest_panel) (`/Game/GEP/Blueprints/UI/WGT_BP_ChestPanel.slot_8_count` _chest_panel) (`/Game/GEP/Blueprints/UI/WGT_BP_ChestPanel.slot_9_count` _chest_panel)))
    (else
      (bind _returnvalue_2 (`|CreateWidget` "/Game/GEP/Blueprints/UI/WGT_BP_InventoryPanel.WGT_BP_InventoryPanel_C"))
      (set `self.inv_panel` _returnvalue_2)
      (set `self.inv_slots` (`|MakeArray` (`/Game/GEP/Blueprints/UI/WGT_BP_InventoryPanel.slot_1` _inv_panel) (`/Game/GEP/Blueprints/UI/WGT_BP_InventoryPanel.slot_2` _inv_panel) (`/Game/GEP/Blueprints/UI/WGT_BP_InventoryPanel.slot_3` _inv_panel) (`/Game/GEP/Blueprints/UI/WGT_BP_InventoryPanel.slot_4` _inv_panel) (`/Game/GEP/Blueprints/UI/WGT_BP_InventoryPanel.slot_5` _inv_panel) (`/Game/GEP/Blueprints/UI/WGT_BP_InventoryPanel.slot_6` _inv_panel) (`/Game/GEP/Blueprints/UI/WGT_BP_InventoryPanel.slot_7` _inv_panel) (`/Game/GEP/Blueprints/UI/WGT_BP_InventoryPanel.slot_8` _inv_panel) (`/Game/GEP/Blueprints/UI/WGT_BP_InventoryPanel.slot_9` _inv_panel) (`/Game/GEP/Blueprints/UI/WGT_BP_InventoryPanel.slot_10` _inv_panel) (`/Game/GEP/Blueprints/UI/WGT_BP_InventoryPanel.slot_11` _inv_panel) (`/Game/GEP/Blueprints/UI/WGT_BP_InventoryPanel.slot_12` _inv_panel) (`/Game/GEP/Blueprints/UI/WGT_BP_InventoryPanel.slot_13` _inv_panel) (`/Game/GEP/Blueprints/UI/WGT_BP_InventoryPanel.slot_14` _inv_panel) (`/Game/GEP/Blueprints/UI/WGT_BP_InventoryPanel.slot_15` _inv_panel) (`/Game/GEP/Blueprints/UI/WGT_BP_InventoryPanel.slot_16` _inv_panel) (`/Game/GEP/Blueprints/UI/WGT_BP_InventoryPanel.slot_17` _inv_panel) (`/Game/GEP/Blueprints/UI/WGT_BP_InventoryPanel.slot_18` _inv_panel) (`/Game/GEP/Blueprints/UI/WGT_BP_InventoryPanel.slot_19` _inv_panel) (`/Game/GEP/Blueprints/UI/WGT_BP_InventoryPanel.slot_20` _inv_panel) (`/Game/GEP/Blueprints/UI/WGT_BP_InventoryPanel.slot_21` _inv_panel) (`/Game/GEP/Blueprints/UI/WGT_BP_InventoryPanel.slot_22` _inv_panel) (`/Game/GEP/Blueprints/UI/WGT_BP_InventoryPanel.slot_23` _inv_panel) (`/Game/GEP/Blueprints/UI/WGT_BP_InventoryPanel.slot_24` _inv_panel) (`/Game/GEP/Blueprints/UI/WGT_BP_InventoryPanel.slot_25` _inv_panel) (`/Game/GEP/Blueprints/UI/WGT_BP_InventoryPanel.slot_26` _inv_panel) (`/Game/GEP/Blueprints/UI/WGT_BP_InventoryPanel.slot_27` _inv_panel) (`/Game/GEP/Blueprints/UI/WGT_BP_InventoryPanel.slot_28` _inv_panel) (`/Game/GEP/Blueprints/UI/WGT_BP_InventoryPanel.slot_29` _inv_panel) (`/Game/GEP/Blueprints/UI/WGT_BP_InventoryPanel.slot_30` _inv_panel) (`/Game/GEP/Blueprints/UI/WGT_BP_InventoryPanel.slot_31` _inv_panel) (`/Game/GEP/Blueprints/UI/WGT_BP_InventoryPanel.slot_32` _inv_panel) (`/Game/GEP/Blueprints/UI/WGT_BP_InventoryPanel.slot_33` _inv_panel) (`/Game/GEP/Blueprints/UI/WGT_BP_InventoryPanel.slot_34` _inv_panel) (`/Game/GEP/Blueprints/UI/WGT_BP_InventoryPanel.slot_35` _inv_panel) (`/Game/GEP/Blueprints/UI/WGT_BP_InventoryPanel.slot_36` _inv_panel)))
      (set `self.slot_counts` (`|MakeArray` (`/Game/GEP/Blueprints/UI/WGT_BP_InventoryPanel.slot_1_count` _inv_panel) (`/Game/GEP/Blueprints/UI/WGT_BP_InventoryPanel.slot_2_count` _inv_panel) (`/Game/GEP/Blueprints/UI/WGT_BP_InventoryPanel.slot_3_count` _inv_panel) (`/Game/GEP/Blueprints/UI/WGT_BP_InventoryPanel.slot_4_count` _inv_panel) (`/Game/GEP/Blueprints/UI/WGT_BP_InventoryPanel.slot_5_count` _inv_panel) (`/Game/GEP/Blueprints/UI/WGT_BP_InventoryPanel.slot_6_count` _inv_panel) (`/Game/GEP/Blueprints/UI/WGT_BP_InventoryPanel.slot_7_count` _inv_panel) (`/Game/GEP/Blueprints/UI/WGT_BP_InventoryPanel.slot_8_count` _inv_panel) (`/Game/GEP/Blueprints/UI/WGT_BP_InventoryPanel.slot_9_count` _inv_panel) (`/Game/GEP/Blueprints/UI/WGT_BP_InventoryPanel.slot_10_count` _inv_panel) (`/Game/GEP/Blueprints/UI/WGT_BP_InventoryPanel.slot_11_count` _inv_panel) (`/Game/GEP/Blueprints/UI/WGT_BP_InventoryPanel.slot_12_count` _inv_panel) (`/Game/GEP/Blueprints/UI/WGT_BP_InventoryPanel.slot_13_count` _inv_panel) (`/Game/GEP/Blueprints/UI/WGT_BP_InventoryPanel.slot_14_count` _inv_panel) (`/Game/GEP/Blueprints/UI/WGT_BP_InventoryPanel.slot_15_count` _inv_panel) (`/Game/GEP/Blueprints/UI/WGT_BP_InventoryPanel.slot_16_count` _inv_panel) (`/Game/GEP/Blueprints/UI/WGT_BP_InventoryPanel.slot_17_count` _inv_panel) (`/Game/GEP/Blueprints/UI/WGT_BP_InventoryPanel.slot_18_count` _inv_panel) (`/Game/GEP/Blueprints/UI/WGT_BP_InventoryPanel.slot_19_count` _inv_panel) (`/Game/GEP/Blueprints/UI/WGT_BP_InventoryPanel.slot_20_count` _inv_panel) (`/Game/GEP/Blueprints/UI/WGT_BP_InventoryPanel.slot_21_count` _inv_panel) (`/Game/GEP/Blueprints/UI/WGT_BP_InventoryPanel.slot_22_count` _inv_panel) (`/Game/GEP/Blueprints/UI/WGT_BP_InventoryPanel.slot_23_count` _inv_panel) (`/Game/GEP/Blueprints/UI/WGT_BP_InventoryPanel.slot_24_count` _inv_panel) (`/Game/GEP/Blueprints/UI/WGT_BP_InventoryPanel.slot_25_count` _inv_panel) (`/Game/GEP/Blueprints/UI/WGT_BP_InventoryPanel.slot_26_count` _inv_panel) (`/Game/GEP/Blueprints/UI/WGT_BP_InventoryPanel.slot_27_count` _inv_panel) (`/Game/GEP/Blueprints/UI/WGT_BP_InventoryPanel.slot_28_count` _inv_panel) (`/Game/GEP/Blueprints/UI/WGT_BP_InventoryPanel.slot_29_count` _inv_panel) (`/Game/GEP/Blueprints/UI/WGT_BP_InventoryPanel.slot_30_count` _inv_panel) (`/Game/GEP/Blueprints/UI/WGT_BP_InventoryPanel.slot_31_count` _inv_panel) (`/Game/GEP/Blueprints/UI/WGT_BP_InventoryPanel.slot_32_count` _inv_panel) (`/Game/GEP/Blueprints/UI/WGT_BP_InventoryPanel.slot_33_count` _inv_panel) (`/Game/GEP/Blueprints/UI/WGT_BP_InventoryPanel.slot_34_count` _inv_panel) (`/Game/GEP/Blueprints/UI/WGT_BP_InventoryPanel.slot_35_count` _inv_panel) (`/Game/GEP/Blueprints/UI/WGT_BP_InventoryPanel.slot_36_count` _inv_panel))))))

(fn `AddItem`
  (params (item_id :type Integer))
  (locals (stacking :type Boolean) (max_stack_index :type Integer))
  (bind _next_available_slot (`self.next_available_slot`))
  (bind _slot_datas (`self.slot_datas`))
  (`/Engine/EditorBlueprintResources/StandardMacros.CompareInt` _next_available_slot (`KismetArrayLibrary.Array_LastIndex` (`self.slot_datas`))
    (:`<`
      (`/Engine/EditorBlueprintResources/StandardMacros.CompareInt` item_id
        (:`>`
          (switch `int` item_id
            (:`Default`
              (set `local.max_stack_index` 0 :!label _label))
            (:`0`
              (goto _label))
            (:`1`
              (goto _label))
            (:`2`
              (goto _label))
            (:`3`
              (goto _label))
            (:`4`
              (goto _label))
            (:`5`
              (goto _label))
            (:`6`
              (goto _label))
            (:`7`
              (goto _label))
            (:`8`
              (goto _label))
            (:`9`
              (goto _label))
            (:`10`
              (set `local.max_stack_index` 1))
            (:`11`
              (set `local.max_stack_index` 2))
            (:`12`
              (goto _label)))
          (for (_array_element _array_index) _slot_datas
            (bind (_id _count) (break `/Game/GEP/Blueprints/Structs/STR_Slot_Data` _array_element))
            (`/Engine/EditorBlueprintResources/StandardMacros.CompareInt` _id item_id
              (:`==`
                (`/Engine/EditorBlueprintResources/StandardMacros.CompareInt` _count (`|GetArrayItem` (`self.max_stack`) (`local.max_stack_index`))
                  (:`<`
                    (bind _output_get (set `local.stacking` true))
                    (break))))))
          (if _output_get
            (`/Engine/EditorBlueprintResources/StandardMacros.IncrementInt` (`.count_5_D2A10951410F7154C4BEE69E93C2DD59` (break `/Game/GEP/Blueprints/Structs/STR_Slot_Data` (`|GetArrayItem` _slot_datas _array_index)))
              (:`  `
                _))
            (else
              (bind _structout (setmembers `/Game/GEP/Blueprints/Structs/STR_Slot_Data` :`StructRef` (`|GetArrayItem` _slot_datas _next_available_slot) :`id` item_id))
              (`/Engine/EditorBlueprintResources/StandardMacros.IncrementInt` (`.count_5_D2A10951410F7154C4BEE69E93C2DD59` (break `/Game/GEP/Blueprints/Structs/STR_Slot_Data` _structout))
                (:`  `
                  _))))
          (`self.UpdateInventory`)
          (`self.UpdateNextAvailableSlot`)
          (`self.UpdateSlotCounts`)
          (`KismetSystemLibrary.PrintText` (`KismetTextLibrary.Conv_IntToText` _next_available_slot)))))))

(fn `CalculateSelectorPosition`
  (locals (local_selected_row :type Integer) (local_selected_column :type Integer))
  (bind _local_selected_column (`local.local_selected_column`))
  (bind _local_selected_row (`local.local_selected_row`))
  (for _ (range 1 (+ (`self.selected_slot`) 1))
    (bind _result (`/Engine/EditorBlueprintResources/StandardMacros.IncrementInt` _local_selected_column)
      (:`  `
        (`/Engine/EditorBlueprintResources/StandardMacros.CompareInt` _result (`self.row_length`)
          (:`==`
            (`/Engine/EditorBlueprintResources/StandardMacros.IncrementInt` _local_selected_row
              (:`  `
                (set `local.local_selected_column` 0))))))))
  (set `self.selected_row` _local_selected_row)
  (set `self.selected_column` _local_selected_column))

(fn `GetCurrentItemId`
  (returns (item_id :type Integer))
  (return (`.id_3_3FB7814F4933E081725AC78D5E72C056` (break `/Game/GEP/Blueprints/Structs/STR_Slot_Data` (`|GetArrayItem` (`self.slot_datas`) (`self.selected_slot`))))))

(fn `InventoryOff`
  (if (`self.chest`)
    (`Widget.RemoveFromParent` (`self.chest_panel`))
    (else
      (`Widget.RemoveFromParent` (`self.inv_panel`)))))

(fn `InventoryOn`
  (if (`self.chest`)
    (`UserWidget.AddToViewport` (`self.chest_panel`) 0)
    (else
      (`UserWidget.AddToViewport` (`self.inv_panel`) 0))))

(fn `MoveSlotSelector`
  (params (direction :type Integer))
  (bind _selected_slot (`self.selected_slot`))
  (bind _selected_row (`self.selected_row`))
  (bind _row_length (`self.row_length`))
  (bind _selected_column (`self.selected_column`))
  (bind _returnvalue (`KismetArrayLibrary.Array_LastIndex` (`self.slot_datas`)))
  (switch `int` direction
    (:`0`
      (`/Engine/EditorBlueprintResources/StandardMacros.CompareInt` _selected_slot
        (:`>`
          (`/Engine/EditorBlueprintResources/StandardMacros.DecrementInt` _selected_slot
            (:`  `
              _)))))
    (:`1`
      (`/Engine/EditorBlueprintResources/StandardMacros.CompareInt` _selected_slot _returnvalue
        (:`<`
          (`/Engine/EditorBlueprintResources/StandardMacros.IncrementInt` _selected_slot
            (:`  `
              _)))))
    (:`2`
      (`/Engine/EditorBlueprintResources/StandardMacros.CompareInt` _selected_slot (- _row_length 1)
        (:`>`
          (set `self.selected_slot` (- _selected_slot _row_length)))))
    (:`3`
      (`/Engine/EditorBlueprintResources/StandardMacros.CompareInt` _selected_slot (+ (- _returnvalue _row_length) 1)
        (:`<`
          (set `self.selected_slot` (+ _selected_slot _row_length))))))
  (`self.CalculateSelectorPosition`)
  (if (`self.chest`)
    (`/Game/GEP/Blueprints/UI/WGT_BP_ChestPanel.UpdateSlotSelector` (`self.chest_panel`) _selected_row _selected_column)
    (else
      (`/Game/GEP/Blueprints/UI/WGT_BP_InventoryPanel.UpdateSlotSelector` (`self.inv_panel`) _selected_row _selected_column))))

(fn `PlaceItem`
  (params (place_location :type "Vector Structure"))
  (bind _returnvalue (`KismetMathLibrary.Conv_VectorToTransform` place_location))
  (switch `int` (`.id_3_3FB7814F4933E081725AC78D5E72C056` (break `/Game/GEP/Blueprints/Structs/STR_Slot_Data` (`|GetArrayItem` (`self.slot_datas`) (`self.selected_slot`))))
    (:`Default`
      (`KismetSystemLibrary.PrintText` "Select an item before trying to place" :!label _label))
    (:`0`
      (goto _label))
    (:`1`
      (`|SpawnActorFromClass` "/Game/GEP/Blueprints/Items/BP_Grass.BP_Grass_C" _returnvalue "Undefined" "MultiplyWithRoot" null null))
    (:`2`
      (`|SpawnActorFromClass` "/Game/GEP/Blueprints/Items/BP_Dirt.BP_Dirt_C" _returnvalue "Undefined" "MultiplyWithRoot" null null))
    (:`3`
      (`|SpawnActorFromClass` "/Game/GEP/Blueprints/Items/BP_Stone.BP_Stone_C" _returnvalue "Undefined" "MultiplyWithRoot" null null))
    (:`4`
      (`|SpawnActorFromClass` "/Game/GEP/Blueprints/Items/BP_Iron.BP_Iron_C" _returnvalue "Undefined" "MultiplyWithRoot" null null))
    (:`5`
      (`|SpawnActorFromClass` "/Game/GEP/Blueprints/Items/BP_Gold.BP_Gold_C" _returnvalue "Undefined" "MultiplyWithRoot" null null))
    (:`6`
      (`|SpawnActorFromClass` "/Game/GEP/Blueprints/Items/BP_Diamond.BP_Diamond_C" _returnvalue "Undefined" "MultiplyWithRoot" null null))
    (:`7`
      (`|SpawnActorFromClass` "/Game/GEP/Blueprints/Items/BP_Emerald.BP_Emerald_C" _returnvalue "Undefined" "MultiplyWithRoot" null null))
    (:`8`
      (`|SpawnActorFromClass` "/Game/GEP/Blueprints/Items/BP_Copper.BP_Copper_C" _returnvalue "Undefined" "MultiplyWithRoot" null null))
    (:`9`
      (`|SpawnActorFromClass` "/Game/GEP/Blueprints/Items/BP_Lapis_Lazuli.BP_Lapis_Lazuli_C" _returnvalue "Undefined" "MultiplyWithRoot" null null))
    (:`10`
      (`|SpawnActorFromClass` "/Game/GEP/Blueprints/Items/BP_Snowball.BP_Snowball_C" _returnvalue "Undefined" "MultiplyWithRoot" null null))
    (:`11`
      (`|SpawnActorFromClass` "/Game/GEP/Blueprints/Items/BP_Sword.BP_Sword_C" _returnvalue "Undefined" "MultiplyWithRoot" null null))
    (:`12`
      (`|SpawnActorFromClass` "/Game/GEP/Blueprints/Items/BP_Coal.BP_Coal_C" _returnvalue "Undefined" "MultiplyWithRoot" null null))))

(fn `RemoveItem`
  (bind _output (`|GetArrayItem` (`self.slot_datas`) (`self.selected_slot`)))
  (bind _result (`/Engine/EditorBlueprintResources/StandardMacros.DecrementInt` (`.count_5_D2A10951410F7154C4BEE69E93C2DD59` (break `/Game/GEP/Blueprints/Structs/STR_Slot_Data` _output)))
    (:`  `
      (`/Engine/EditorBlueprintResources/StandardMacros.CompareInt` _result
        (:`>`
          _)
        (:`==`
          (setmembers `/Game/GEP/Blueprints/Structs/STR_Slot_Data` :`StructRef` _output :`id` 0)))
      (`self.UpdateInventory`)
      (`self.UpdateNextAvailableSlot`)
      (`self.UpdateSlotCounts`))))

(fn `UpdateInventory`
  (for (_array_element _array_index) (`self.slot_datas`)
    (switch `int` (`.id_3_3FB7814F4933E081725AC78D5E72C056` (break `/Game/GEP/Blueprints/Structs/STR_Slot_Data` _array_element))
      (:`Default`
        (set `self.icon_texture` null :!label _label)
        (set `self.icon_opacity` 0.0))
      (:`0`
        (goto _label))
      (:`1`
        (set `self.icon_texture` "/Game/GEP/Images/grass_icon.grass_icon")
        (set `self.icon_opacity` 1.0 :!label _label_2))
      (:`2`
        (set `self.icon_texture` "/Game/GEP/Images/dirt_icon.dirt_icon")
        (goto _label_2))
      (:`3`
        (set `self.icon_texture` "/Game/GEP/Images/stone_icon.stone_icon")
        (goto _label_2))
      (:`4`
        (set `self.icon_texture` "/Game/GEP/Images/iron_icon.iron_icon")
        (goto _label_2))
      (:`5`
        (set `self.icon_texture` "/Game/GEP/Images/gold_icon.gold_icon")
        (goto _label_2))
      (:`6`
        (set `self.icon_texture` "/Game/GEP/Images/diamond_icon.diamond_icon")
        (goto _label_2))
      (:`7`
        (set `self.icon_texture` "/Game/GEP/Images/emerald_icon.emerald_icon")
        (goto _label_2))
      (:`8`
        (set `self.icon_texture` "/Game/GEP/Images/copper_icon.copper_icon")
        (goto _label_2))
      (:`9`
        (set `self.icon_texture` "/Game/GEP/Images/lapis_lazuli_icon.lapis_lazuli_icon")
        (goto _label_2))
      (:`10`
        (set `self.icon_texture` "/Game/GEP/Images/snowball_icon.snowball_icon")
        (goto _label_2))
      (:`11`
        (set `self.icon_texture` "/Game/GEP/Images/sword_icon.sword_icon")
        (goto _label_2))
      (:`12`
        (set `self.icon_texture` "/Game/GEP/Images/coal_icon.coal_icon")
        (goto _label_2)))
    (bind _output (`|GetArrayItem` (`self.inv_slots`) _array_index))
    (`Image.SetBrushFromTexture` _output (`self.icon_texture`) false)
    (`Image.SetOpacity` _output (`self.icon_opacity`))))

(fn `UpdateNextAvailableSlot`
  (for (_array_element _array_index) (`self.slot_datas`)
    (`/Engine/EditorBlueprintResources/StandardMacros.CompareInt` (`.id_3_3FB7814F4933E081725AC78D5E72C056` (break `/Game/GEP/Blueprints/Structs/STR_Slot_Data` _array_element))
      (:`==`
        (set `self.next_available_slot` _array_index)
        (break)))))

(fn `UpdateSlotCounts`
  (for (_array_element _array_index) (`self.slot_datas`)
    (bind ((`count_5_D2A10951410F7154C4BEE69E93C2DD59` _count)) (break `/Game/GEP/Blueprints/Structs/STR_Slot_Data` _array_element))
    (bind _output (`|GetArrayItem` (`self.slot_counts`) _array_index))
    (set `TextBlock.Text` (`KismetTextLibrary.Conv_IntToText` _count) _output)
    (`/Engine/EditorBlueprintResources/StandardMacros.CompareInt` _count 1
      (:`>`
        (`Widget.SetVisibility` _output "Visible"))
      (:`==`
        (`Widget.SetVisibility` _output "Hidden" :!label _label))
      (:`<`
        (goto _label)))))